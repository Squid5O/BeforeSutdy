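; BP_Enemy is an enemy actor that flies in a straight line and damages the player on contact.
; At BeginPlay it picks a fixed direction, 30% toward the player and otherwise forward, then Tick sweeps it along that direction and faces it that way.
; When an overlap with BP_Player ends, it spawns an explosion, deals damage and destroys itself.
; At zero health it also destroys the player, shows WBP_GameOver and pauses the game.
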(event EventBeginPlay
  ;[1 1 1] 태어날 떄 이동할 방향을 기억하고 싶 다. 30% 확률로 프레이어 방향 나머지 확률로 앞방향으로 하고 싶다.
  (if (< (Math|Random|RandomIntegerinRange 0 9) 3)
    (Variables|Default|Setdirection (Math|Vector|Normalize (- (Transformation|GetActorLocation (Game|Player|GetPlayerPawn 0)) (Transformation|GetActorLocation))))
    (else
      (Variables|Default|Setdirection (Transformation|GetActorForwardVector)))))

(event Collision|EventActorBeginOverlap
  (params (OtherActor :type Actor%20Object%20Reference))
  (Development|PrintString (Utilities|GetDisplayName OtherActor)))

(event EventTick
  (params (DeltaSeconds :type Float%20%28single-precision%29))
  (Utilities|FlowControl|Sequence
    (:then_0
      ;[1 1 1] 기억하고 있는 앞 방향으로 계속 나아가라
      (Transformation|SetActorLocation (+ (Transformation|GetActorLocation) (* (Variables|Default|Getdirection) (Variables|Default|Getspeed) (Utilities|Time|GetWorldDeltaSeconds))) true false))
    (:then_1
      ;[1 1 1] 이동하는 방향으로 회전하고 싶엉
      (Transformation|SetActorRotation (Math|Rotator|MakeRotfromXZ (Variables|Default|Getdirection) (Transformation|GetActorUpVector))))))

(event Collision|EventActorEndOverlap
  (params (OtherActor :type Actor%20Object%20Reference))
  (bind _returnvalue (Game|GetPlayerController 0))
  ;[1 1 1] 충돌한 상대방이 플레이어라면 너 체력 1 달고 만약 체력이 0이면 죽고, 나 죽음 ㅅㄱ
  (bind _asbp_player (Utilities|Casting|CastToBP_Player OtherActor))
  (Effects|SpawnEmitteratLocation "/Game/StarterContent/Particles/P_Explosion.P_Explosion" (Transformation|GetActorLocation))
  (bind _result_hp (Default|MyApplyDamage _asbp_player 1))
  (if (<= _result_hp 0)
    (Actor|DestroyActor OtherActor)
    (Actor|DestroyActor)
    (bind _returnvalue_2 (UserInterface|CreateWidget "/Game/UI/WBP_GameOver.WBP_GameOver_C"))
    (UserInterface|Viewport|AddtoViewport _returnvalue_2 0)
    (Variables|/Script/Engine.PlayerController|SetbShowMouseCursor _returnvalue true)
    (Input|SetInputModeUIOnly _returnvalue 0 "DoNotLock" false)
    (Game|SetGamePaused true)
    (else
      (Actor|DestroyActor))))

(fn ConstructionScript)