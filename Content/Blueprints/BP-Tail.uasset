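; BP-Tail is an actor that continuously chases a Target actor, defaulting to the player.
; On BeginPlay, an invalid Target is replaced with the actor returned by GetActorOfClass for BP_Player.
; Each Tick moves it straight toward the Target at Speed, scaled by delta time.
; Movement uses SetActorLocation without sweep, with no stopping distance or rotation update.
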(event EventBeginPlay
  ;[1 1 1] 태너알 때 목적지가 있찌 않다면 유하지 않다면 중니공 플레이를 주인공 플레이러를 목적지로 하고싶다능
  (Utilities|IsValid (Variables|Default|Gettarget)
    (:Is%20Not%20Valid
      (bind _returnvalue (Actor|GetActorOfClass "/Game/Blueprints/BP_Player.BP_Player_C"))
      (Variables|Default|Settarget _returnvalue))))

(event Collision|EventActorBeginOverlap
  (params (OtherActor :type Actor%20Object%20Reference)))

(event EventTick
  (params (DeltaSeconds :type Float%20%28single-precision%29))
  ;[1 1 1] 살아가면서 목적지를 향해서 계속 이동 하고 싶어.
  (Transformation|SetActorLocation (+ (Transformation|GetActorLocation) (* (Math|Vector|Normalize (- (Transformation|GetActorLocation (Variables|Default|Gettarget)) (Transformation|GetActorLocation))) (Variables|Default|Getspeed) (Utilities|Time|GetWorldDeltaSeconds))) false false))

(fn ConstructionScript)