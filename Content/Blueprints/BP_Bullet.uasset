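; BP_Bullet is a shooting-game projectile that destroys enemies and adds to the score.
; Tick moves it along its forward vector at Speed, scaled by delta seconds, without sweeping.
; When an overlap with a BP_Enemy ends (not begins), it spawns an explosion, destroys both actors, increments Score on BP_ShootingGameModeBase and plays a sound.
; The Trasnlate helper repeats the movement math but is never run.
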(event EventBeginPlay)

(event Collision|EventActorBeginOverlap
  (params (OtherActor :type Actor%20Object%20Reference)))

(event EventTick
  (params (DeltaSeconds :type Float%20%28single-precision%29))
  ;[1 1 1] 살아가면서 앞방향으로 계속 이동하고 싶다.
  (Transformation|SetActorLocation (+ (Transformation|GetActorLocation) (* (Transformation|GetActorForwardVector) (Variables|Default|Getspeed) (Utilities|Time|GetWorldDeltaSeconds))) false false))

(event Collision|EventActorEndOverlap
  (params (OtherActor :type Actor%20Object%20Reference))
  ;[1 1 1] 충돌한 상대방이 플레이어라면 너죽고 나죽고 하고 싶다,
  (bind _asbp_enemy (Utilities|Casting|CastToBP_Enemy OtherActor))
  (Effects|SpawnEmitteratLocation "/Game/StarterContent/Particles/P_Explosion.P_Explosion" (Transformation|GetActorLocation))
  (Actor|DestroyActor _asbp_enemy)
  (Actor|DestroyActor)
  (bind _asbp_shooting_game_mode_base (Utilities|Casting|CastToBP_ShootingGameModeBase (Game|GetGameMode)))
  (Math|Integer|IncrementInt (Variables|/Game/Blueprints/BP_ShootingGameModeBase.BP_ShootingGameModeBase_C|GetScore _asbp_shooting_game_mode_base)
    (:%20%20
      (Audio|PlaySound2D "/Game/sound/Audio_Explosion.Audio_Explosion" 1.0 1.0 0.0 0 0))))

(fn ConstructionScript)

(fn Trasnlate
  (params (Direction :type Vector) (Speed :type Float%20%28double-precision%29))
  ;[1 1 1] P = P0 + velocity(dir*speed)*deltaSecond(t)
  (Transformation|SetActorLocation (+ (Transformation|GetActorLocation) (* Direction Speed (Utilities|Time|GetWorldDeltaSeconds))) false false))