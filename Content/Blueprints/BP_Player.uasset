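; Player actor for a shooter that moves on the world YZ plane and toggles automatic fire with the fire input.
; Each Tick, normalized horizontal and vertical input drives a custom swept translate, and an accumulated timer spawns bullets while auto-fire is on.
; MakeBullet spawns BP_Bullet at the Arrow component and plays a shot sound.
; HP starts at MaxHP, and MyApplyDamage subtracts damage and returns the remainder.
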(event Custom|MakeBullet
  (bind _arrow (Variables|Default|GetArrow))
  (bind _returnvalue (Transformation|GetWorldTransform _arrow))
  (Game|SpawnActorfromClass "/Game/Blueprints/BP_Bullet.BP_Bullet_C" (Math|Transform|MakeTransform (.location _returnvalue) (.rotation _returnvalue) "1.000000,1.000000,1.000000") "Undefined" "MultiplyWithRoot" 0 0)
  (Audio|PlaySound2D "/Game/sound/Audio_Bullet.Audio_Bullet" 1.0 1.0 0.0 0 0))

(event EventBeginPlay
  ;[1 1 1] 플레이어가 태어날때 HP에 MaxHP값을 Set 하고 싶다.
  (Variables|Default|SetHP (Variables|Default|GetMaxHP)))

(event Collision|EventActorBeginOverlap
  (params (OtherActor :type Actor%20Object%20Reference))
  ;[1 1 1] translate
)

(event EventTick
  (params (DeltaSeconds :type Float%20%28single-precision%29))
  ;[1 1 1] translate
  (Utilities|FlowControl|Sequence
    (:then_0
      (CallFunction|Trasnlate (Math|Vector|Normalize (Math|Vector|MakeVector 0.0 (Input|AxisValues|GetHorizontal) (Input|AxisValues|GetVertical))) (Variables|Default|Getspeed)))
    (:then_1
      ;[1 1 1] autoFIre
      (if (Variables|Default|GetIsAutoFire)
        ;;[1 1 1] 시간이 흐르다가
        (Variables|Default|SetCurrentTIme (+ (Variables|Default|GetCurrentTIme) (Utilities|Time|GetWorldDeltaSeconds)))
        ;;[1 1 1] 현재 시간이 총 쏠 시간이 되었따면
        (if (>= (Variables|Default|GetCurrentTIme) (Variables|Default|GetAutoFIreTime))
          (CallFunction|MakeBullet)
          (Variables|Default|SetCurrentTIme 0.0))))))

(event Input|ActionEvents|InputActionfire
  (params (Key :type Key%20Structure :default "None"))
  (:Pressed
    (if (Variables|Default|GetIsAutoFire)
      (Variables|Default|SetIsAutoFire false)
      (else
        (Variables|Default|SetIsAutoFire true)
        (Variables|Default|SetCurrentTIme 0.0)
        (CallFunction|MakeBullet)))))

(event Input|AxisEvents|InputAxisHorizontal
  (params (AxisValue :type Float%20%28single-precision%29))
  ;[1 1 1] translate
)

(fn ConstructionScript)

(fn Trasnlate
  (params (Direction :type Vector) (Speed :type Float%20%28double-precision%29))
  ;[1 1 1] P = P0 + velocity(dir*speed)*deltaSecond(t)
  (Transformation|SetActorLocation (+ (Transformation|GetActorLocation) (* Direction Speed (Utilities|Time|GetWorldDeltaSeconds))) true false))

(fn MyApplyDamage
  (params (Damage :type Integer))
  (Variables|Default|SetHP (- (Variables|Default|GetHP) Damage))
  (return (Variables|Default|GetHP)))