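; BP_EnmeyManger is a spawner actor that creates BP_Enemy instances at a regular interval.
; BeginPlay starts a looping timer on SpawnTIme that calls SpawnEnemy.
; SpawnEnemy spawns at the Spawn component's world location and rotation, always ignoring collision, and only while player pawn 0 is valid.
; Alternative Delay, delta-time accumulator and Timeline approaches remain in the graph but are disconnected.
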(event Custom|SpawnEnemy
  (bind _spawn (Variables|Default|GetSpawn))
  (bind _returnvalue (Transformation|GetWorldTransform _spawn))
  (Utilities|IsValid (Game|Player|GetPlayerPawn 0)
    (:Is%20Valid
      (Game|SpawnActorfromClass "/Game/Blueprints/BP_Enemy.BP_Enemy_C" (Math|Transform|MakeTransform (.location _returnvalue) (.rotation _returnvalue) "1.000000,1.000000,1.000000") "AlwaysSpawn" "MultiplyWithRoot" 0 0))))

(event EventBeginPlay
  ;[1 1 1] timer?
  (Utilities|Time|SetTimerbyEvent (delegate Custom|SpawnEnemy) (Variables|Default|GetSpawnTIme) true))

(event Collision|EventActorBeginOverlap
  (params (OtherActor :type Actor%20Object%20Reference)))

(event EventTick
  (params (DeltaSeconds :type Float%20%28single-precision%29)))

(fn ConstructionScript)